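; A game mode for a coin-collecting level that is won when every coin has been hit.
; On BeginPlay it spawns one Coin at each of the first CoinsNumber actors tagged SpawnPoint, in lookup order.
; OnCoinHit counts hits and prints how many coins remain, or on the last one prints a win message and reloads the current level after a short delay.
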(event Custom|OnCoinHit
  (Variables|Default|SetCurrentCoinsHitNumber (+ (Variables|Default|GetCurrentCoinsHitNumber) 1))
  (if (== (Variables|Default|GetCurrentCoinsHitNumber) (Variables|Default|GetCoinsNumber))
    (Development|PrintString "YOU WON" true true "(R=0.000000,G=0.660000,B=1.000000,A=1.000000)" 1e+01)
    (Utilities|FlowControl|Delay 5.0)
    (bind _returnvalue (Game|GetCurrentLevelName true))
    (Game|OpenLevel(byName) (Utilities|String|StringToName _returnvalue))
    (else
      (Development|PrintString (Utilities|String|ToString(Integer) (- (Variables|Default|GetCoinsNumber) (Variables|Default|GetCurrentCoinsHitNumber)))) ; Coins to colect
    )))

(event EventBeginPlay
  (bind _outactors (Actor|GetAllActorswithTag "SpawnPoint"))
  (for _index (range 0 (- (Variables|Default|GetCoinsNumber) 1))
    (Game|SpawnActorfromClass "/Game/Blueprints/Coin.Coin_C" (Math|Conversions|ToTransform(Vector) (Transformation|GetActorLocation (Utilities|Array|Get(acopy) _outactors _index))) "Undefined" "MultiplyWithRoot" 0 0)))

(fn ConstructionScript)